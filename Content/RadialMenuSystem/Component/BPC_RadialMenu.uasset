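; Component that runs a configurable 2 to 6 option radial menu for triggering third-person character abilities.
; Opening creates the matching wheel widget, sets input mode and applies slow motion.
; Gamepad stick or mouse axes feed the widget, while any key press detects gamepad use and, without AutoSelect, handles select and cancel.
; Closing restores time and, unless cancelled, calls the hovered option's ability when auto-selecting or selected.
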(event Custom|Open%20Radial%20Menu
  (bind _number_of_options (Variables|Customizing|GetNumber%20of%20Options))
  ;[0.5207 0.6194 1] Open and Close Radial Menu
  (Variables|PrivateVariables|SetIsOpen true)
  (switch Utilities|FlowControl|Switch|SwitchonE_NumberOfSelections _number_of_options
    (:NewEnumerator4
      (bind _outputpin (|2PieceWheel)))
    (:NewEnumerator3
      (bind _outputpin_2 (|3PieceWheel)))
    (:NewEnumerator0
      (bind _outputpin_3 (|4PieceWheel)))
    (:NewEnumerator1
      (bind _outputpin_4 (|5PieceWheel)))
    (:NewEnumerator2
      (bind _outputpin_5 (|6PieceWheel))))
  (|InputMode (Utilities|Select :Index _number_of_options :NewEnumerator4 _outputpin :NewEnumerator3 _outputpin_2 :NewEnumerator0 _outputpin_3 :NewEnumerator1 _outputpin_4 :NewEnumerator2 _outputpin_5))
  (|SlowMotion)
  (|InitializeWidget))

(event Custom|Close%20Radial%20Menu
  ;[0.5207 0.6194 1] Open and Close Radial Menu
  (if (Variables|PrivateVariables|GetIsOpen)
    (Variables|PrivateVariables|SetIsOpen false)
    (Utilities|FlowControl|Sequence
      (:then_0
        (|CloseMenu))
      (:then_1
        (if (or (Variables|Customizing|GetAuto%20Select) (Variables|PrivateVariables|GetSelected))
          (if (Variables|PrivateVariables|GetCancelMenu)
            (Variables|PrivateVariables|SetCancelMenu false)
            (else
              (|SelectButtonWithoutPressing))))))))

(event Custom|Top%20Left%20Function
  ;[1 0.7225 0.2854] Set up each button and what they should do here.
  ;;[1 1 1] Insert your own Character functions here. (Anything goes from making this an emote wheel to letting each button equipdifferent guns
  (Default|TopLeftAbility (Variables|Character|GetChar%20Ref)))

(event Custom|Top%20Right%20Function
  ;[1 0.7225 0.2854] Set up each button and what they should do here.
  ;;[1 1 1] Insert your own Character functions here. (Anything goes from making this an emote wheel to letting each button equipdifferent guns
  (Default|TopRightAbility (Variables|Character|GetChar%20Ref)))

(event Custom|Bottom%20Left%20Function
  ;[1 0.7225 0.2854] Set up each button and what they should do here.
  ;;[1 1 1] Insert your own Character functions here. (Anything goes from making this an emote wheel to letting each button equipdifferent guns
  (Default|BottomLeftAbility (Variables|Character|GetChar%20Ref)))

(event Custom|Bottom%20Right%20Function
  ;[1 0.7225 0.2854] Set up each button and what they should do here.
  ;;[1 1 1] Insert your own Character functions here. (Anything goes from making this an emote wheel to letting each button equipdifferent guns
  (Default|BottomRightAbility (Variables|Character|GetChar%20Ref)))

(event Custom|Bottom%20Middle
  ;[1 0.7225 0.2854] Set up each button and what they should do here.
  ;;[0.9428 1 0] Only used on 5 or 6 piece menu
  (Default|BottomMiddleAbility (Variables|Character|GetChar%20Ref)))

(event Custom|Top%20Middle
  ;[1 0.7225 0.2854] Set up each button and what they should do here.
  ;;[0.3813 0.4072 0] Only Used in 6 piece menu
  (Default|TopMiddleAbility (Variables|Character|GetChar%20Ref)))

(event EventTick
  (params (DeltaSeconds :type Float%20%28single-precision%29))
  ;[0.7032 1 0.5462] Mouse Support
  (switch Utilities|FlowControl|Switch|SwitchonE_NumberOfSelections (Variables|Customizing|GetNumber%20of%20Options)
    (:NewEnumerator4
      (|2PieceAxisValues (stale Input|MouseEvents|MouseY _output_get) (stale Input|MouseEvents|MouseX _output_get)))
    (:NewEnumerator3
      (|3PieceAxisValues (stale Input|MouseEvents|MouseY _output_get) (stale Input|MouseEvents|MouseX _output_get)))
    (:NewEnumerator0
      (|4PieceAxisValues (stale Input|MouseEvents|MouseY _output_get) (stale Input|MouseEvents|MouseX _output_get)))
    (:NewEnumerator1
      (|5PieceAxisValues (stale Input|MouseEvents|MouseY _output_get) (stale Input|MouseEvents|MouseX _output_get)))
    (:NewEnumerator2
      (|6PieceAxisValues (stale Input|MouseEvents|MouseY _output_get) (stale Input|MouseEvents|MouseX _output_get)))))

(event EventBeginPlay
  ;[0.7074 0.5751 1] Event Begin Play
  (Utilities|FlowControl|Sequence
    (:then_0
      (|CharacterCall))
    (:then_1
      (|ControllerPreferencesetup))
    (:then_2
      (|MousePreferencesetup))))

(event Input|GamepadEvents|GamepadLeftY
  (params (AxisValue :type Float%20%28single-precision%29))
  ;[0.5311 0.9901 1] Controller Support
  ;;[0.3534 0.9701 1] Left Stick
  (if (not (Variables|PrivateVariables|GetRight%20Stick))
    (if (Variables|PrivateVariables|GetGamePad%20In%20Use)
      (bind _output_get (Variables|PrivateVariables|SetGamePad%20Y%20Axis%20Value AxisValue))
      (switch Utilities|FlowControl|Switch|SwitchonE_NumberOfSelections (Variables|Customizing|GetNumber%20of%20Options)
        (:NewEnumerator4
          (|2PieceAxisValues_3 _output_get (stale Input|GamepadEvents|GamepadLeftX _output_get)))
        (:NewEnumerator3
          (|3PieceAxisValues_3 _output_get (stale Input|GamepadEvents|GamepadLeftX _output_get)))
        (:NewEnumerator0
          (|4PieceAxisValues_3 _output_get (stale Input|GamepadEvents|GamepadLeftX _output_get)))
        (:NewEnumerator1
          (|5PieceAxisValues_3 _output_get (stale Input|GamepadEvents|GamepadLeftX _output_get)))
        (:NewEnumerator2
          (|6PieceAxisValues_3 _output_get (stale Input|GamepadEvents|GamepadLeftX _output_get)))))))

(event Input|GamepadEvents|GamepadLeftX
  (params (AxisValue :type Float%20%28single-precision%29))
  ;[0.5311 0.9901 1] Controller Support
  ;;[0.3534 0.9701 1] Left Stick
  (if (not (Variables|PrivateVariables|GetRight%20Stick))
    (if (Variables|PrivateVariables|GetGamePad%20In%20Use)
      (bind _output_get (Variables|PrivateVariables|SetGamePad%20X%20Axis%20Value AxisValue))
      (switch Utilities|FlowControl|Switch|SwitchonE_NumberOfSelections (Variables|Customizing|GetNumber%20of%20Options)
        (:NewEnumerator4
          (|2PieceAxisValues_3 (stale Input|GamepadEvents|GamepadLeftY _output_get) _output_get))
        (:NewEnumerator3
          (|3PieceAxisValues_3 (stale Input|GamepadEvents|GamepadLeftY _output_get) _output_get))
        (:NewEnumerator0
          (|4PieceAxisValues_3 (stale Input|GamepadEvents|GamepadLeftY _output_get) _output_get))
        (:NewEnumerator1
          (|5PieceAxisValues_3 (stale Input|GamepadEvents|GamepadLeftY _output_get) _output_get))
        (:NewEnumerator2
          (|6PieceAxisValues_3 (stale Input|GamepadEvents|GamepadLeftY _output_get) _output_get))))))

(event Input|MouseEvents|MouseY
  (params (AxisValue :type Float%20%28single-precision%29))
  ;[0.7032 1 0.5462] Mouse Support
  (if (not (Variables|PrivateVariables|GetHoverAndClick))
    (if (not (Variables|PrivateVariables|GetGamePad%20In%20Use))
      (bind _output_get (Variables|PrivateVariables|SetGamePad%20Y%20Axis%20Value (* AxisValue (Variables|Customizing|GetMouse%20Sensitivity)))))))

(event Input|GamepadEvents|GamepadRightX
  (params (AxisValue :type Float%20%28single-precision%29))
  ;[0.5311 0.9901 1] Controller Support
  ;;[0.51 0.9801 1] Right Stick
  (if (Variables|PrivateVariables|GetRight%20Stick)
    (if (Variables|PrivateVariables|GetGamePad%20In%20Use)
      (bind _output_get (Variables|PrivateVariables|SetGamePad%20X%20Axis%20Value AxisValue))
      (switch Utilities|FlowControl|Switch|SwitchonE_NumberOfSelections (Variables|Customizing|GetNumber%20of%20Options)
        (:NewEnumerator4
          (|2PieceAxisValues_2 (stale Input|GamepadEvents|GamepadRightY _output_get) _output_get))
        (:NewEnumerator3
          (|3PieceAxisValues_2 (stale Input|GamepadEvents|GamepadRightY _output_get) _output_get))
        (:NewEnumerator0
          (|4PieceAxisValues_2 (stale Input|GamepadEvents|GamepadRightY _output_get) _output_get))
        (:NewEnumerator1
          (|5PieceAxisValues_2 (stale Input|GamepadEvents|GamepadRightY _output_get) _output_get))
        (:NewEnumerator2
          (|6PieceAxisValues_2 (stale Input|GamepadEvents|GamepadRightY _output_get) _output_get))))))

(event Input|GamepadEvents|GamepadRightY
  (params (AxisValue :type Float%20%28single-precision%29))
  ;[0.5311 0.9901 1] Controller Support
  ;;[0.51 0.9801 1] Right Stick
  (if (Variables|PrivateVariables|GetRight%20Stick)
    (if (Variables|PrivateVariables|GetGamePad%20In%20Use)
      (bind _output_get (Variables|PrivateVariables|SetGamePad%20Y%20Axis%20Value (* AxisValue -1.0)))
      (switch Utilities|FlowControl|Switch|SwitchonE_NumberOfSelections (Variables|Customizing|GetNumber%20of%20Options)
        (:NewEnumerator4
          (|2PieceAxisValues_2 _output_get (stale Input|GamepadEvents|GamepadRightX _output_get)))
        (:NewEnumerator3
          (|3PieceAxisValues_2 _output_get (stale Input|GamepadEvents|GamepadRightX _output_get)))
        (:NewEnumerator0
          (|4PieceAxisValues_2 _output_get (stale Input|GamepadEvents|GamepadRightX _output_get)))
        (:NewEnumerator1
          (|5PieceAxisValues_2 _output_get (stale Input|GamepadEvents|GamepadRightX _output_get)))
        (:NewEnumerator2
          (|6PieceAxisValues_2 _output_get (stale Input|GamepadEvents|GamepadRightX _output_get)))))))

(event Input|MouseEvents|MouseX
  (params (AxisValue :type Float%20%28single-precision%29))
  ;[0.7032 1 0.5462] Mouse Support
  (if (not (Variables|PrivateVariables|GetHoverAndClick))
    (if (not (Variables|PrivateVariables|GetGamePad%20In%20Use))
      (bind _output_get (Variables|PrivateVariables|SetGamePad%20X%20Axis%20Value (* AxisValue (Variables|Customizing|GetMouse%20Sensitivity)))))))

(event Input|KeyboardEvents|AnyKey
  (params (Key :type Key%20Structure :default "None"))
  (bind _auto_select (Variables|Customizing|GetAuto%20Select))
  (bind _widget_4_piece (Variables|PrivateVariables|GetWidget%204%20Piece))
  ;[1 0.555 0.7966] Check GamePad
  (:Pressed
    (Utilities|FlowControl|Sequence
      (:then_0
        (bind _output_get (Variables|PrivateVariables|SetGamePad%20In%20Use (Class|KismetInputLibrary|KeyIsGamepadKey Key)))
        (Utilities|IsValid _widget_4_piece
          (:Is%20Valid
            (Variables|/Game/RadialMenuSystem/Widget/BPW_RadialWidget4Piece.BPW_RadialWidget4Piece_C|SetGamePad%20In%20Use _widget_4_piece _output_get))))
      (:then_1
        ;;[1 1 1] Cancel Buttons
        (if (not _auto_select)
          (if (or (== Key (Variables|Input|GetCancelButtonKeyBoard)) (== Key (Variables|Input|GetCancelButtonGamePad)))
            (Variables|PrivateVariables|SetSelected true)
            (Variables|PrivateVariables|SetCancelMenu true)
            (CallFunction|CloseRadialMenu))))
      (:then_2
        ;;[1 1 1] Select Buttons
        (if (not _auto_select)
          (if (or (== Key (Variables|Input|GetSelectButtonKeyBoard)) (== Key (Variables|Input|GetSelectButtonGamePad)))
            (Variables|PrivateVariables|SetSelected true)
            (CallFunction|CloseRadialMenu)))))))